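; Actor component that moves its owner along the spline of a referenced SplinePath actor.
; BeginPlay caches that spline once both references are valid.
; Each tick sets the owner's world location and rotation from the spline at SplineTime, without constant velocity, then advances SplineTime by delta time over Duration.
; The graph has no clamping, looping or end-of-path handling.
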(event EventBeginPlay
  (bind _splinepath (Variables|Default|GetSplinePath))
  (Utilities|IsValid _splinepath
    (:Is%20Valid
      (Utilities|IsValid (Variables|/Game/TeacherContent/Blueprints/BP_SplinePath.BP_SplinePath_C|GetSpline _splinepath)
        (:Is%20Valid
          (Variables|Default|SetSpline (Variables|/Game/TeacherContent/Blueprints/BP_SplinePath.BP_SplinePath_C|GetSpline _splinepath)))))))

(event EventTick
  (params (DeltaSeconds :type Float%20%28single-precision%29))
  (bind _spline (Variables|Default|GetSpline))
  (Utilities|IsValid (Variables|Default|GetSpline)
    (:Is%20Valid
      (Utilities|FlowControl|Sequence
        (:then_0
          (Transformation|SetActorLocationAndRotation (Components|GetOwner) (Spline|GetLocationatTime _spline (Variables|Default|GetSplineTime) "World" false) (Class|SplineComponent|GetRotationatTime _spline (Variables|Default|GetSplineTime) "World" false)))
        (:then_1
          (Variables|Default|SetSplineTime (+ (Variables|Default|GetSplineTime) (/ DeltaSeconds (Variables|Default|GetDuration)))))))))