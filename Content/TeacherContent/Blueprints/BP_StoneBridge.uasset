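; Stone bridge that assembles from scattered stones when a neecVRPawn first overlaps it.
; BeginPlay stores each stone's placed transform as target, lowers it by a random height with random rotation, and picks a curve-weighted random duration.
; Once triggered, Tick moves stones home with sinusoidal ease-out.
; The progress update reads the first loop's index, so stones share the last one's timing despite per-stone durations.
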(event EventBeginPlay
  (bind _starttransforms (Variables|Default|GetStartTransforms))
  (for _array_element (Variables|Default|GetStones)
    (Utilities|Array|Add (Variables|Default|GetTargetTransforms) (Transformation|GetActorTransform _array_element))
    (bind _returnvalue (Utilities|Array|Add _starttransforms (Math|Transform|MakeTransform (Math|Vector|MakeVector (.x (.Location (Math|Transform|BreakTransform (Transformation|GetActorTransform _array_element)))) (.y (.Location (Math|Transform|BreakTransform (Transformation|GetActorTransform _array_element)))) (- (.z (.Location (Math|Transform|BreakTransform (Transformation|GetActorTransform _array_element)))) (Math|Random|RandomFloatinRange (Variables|Default|GetHeightMin) (Variables|Default|GetHeightMax)))) (Math|Random|RandomRotator true) (.Scale (Math|Transform|BreakTransform (Transformation|GetActorTransform _array_element))))))
    (Transformation|SetActorTransform _array_element (Utilities|Array|Get(acopy) _starttransforms _returnvalue))
    (Utilities|Array|Add (Variables|Default|GetTransitionTime) (Math|Float|Lerp (Variables|Default|GetTransitionTimeMin) (Variables|Default|GetTransitionTimeMax) (Math|Curves|GetFloatValue (Variables|Default|GetDistributionCurve) (Math|Random|RandomFloat))))
    (Utilities|Array|Add (Variables|Default|GetCurrentTransitionTime) 0.0)))

(event Collision|EventActorBeginOverlap
  (params (OtherActor :type Actor%20Object%20Reference))
  (if (not (Variables|Default|GetTransitionStarted))
    (bind _asneec_vrpawn (Utilities|Casting|CastToneecVRPawn OtherActor))
    (Variables|Default|SetTransitionStarted true)
    (Development|PrintString (Utilities|GetDisplayName _asneec_vrpawn))))

(event EventTick
  (params (DeltaSeconds :type Float%20%28single-precision%29))
  (bind _currenttransitiontime (Variables|Default|GetCurrentTransitionTime))
  (if (Variables|Default|GetTransitionStarted)
    (for (_array_element _array_index) (Variables|Default|GetStones)
      (Transformation|SetActorTransform _array_element (Math|Interpolation|Ease "SinusoidalOut" (Utilities|Array|Get(acopy) (Variables|Default|GetCurrentTransitionTime) _array_index) (Utilities|Array|Get(acopy) (Variables|Default|GetStartTransforms) _array_index) (Utilities|Array|Get(acopy) (Variables|Default|GetTargetTransforms) _array_index))))
    (for (_ _array_index_2) _currenttransitiontime
      (Utilities|Array|SetArrayElem _currenttransitiontime _array_index_2 (Math|Float|Clamp(Float) (+ (Utilities|Array|Get(acopy) (Variables|Default|GetCurrentTransitionTime) _array_index) (* DeltaSeconds (/ 1.0 (Utilities|Array|Get(acopy) (Variables|Default|GetTransitionTime) _array_index)))))))))

(fn ConstructionScript)